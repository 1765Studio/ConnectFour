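; BP_PickableItem is a world item actor that can be looked at and picked up into an inventory.
; On BeginPlay it reads its data table row to set name, description, mesh and uniform scale, writing each of the mesh's materials to slot 0.
; LookAt returns the description and name.
; InteractWith adds the name and quantity to the interactor's InventoryComponent, then destroys the actor.
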(event `self.ReceiveBeginPlay`
  (bind (_itemdata_datatable _itemdata_rowname) (break `DataTableRowHandle` (`self.ItemData`)))
  (bind _cube (`self.Cube`))
  (bind _returnvalue (`|GetDataTableRow` _itemdata_datatable _itemdata_rowname)
    (:`then`
      (set `self.ItemName` (`.RowName` (break `DataTableRowHandle` (`self.ItemData`))))
      (bind (_itemlongname _itemdescription _thumbnail _mesh _value _stackable_ _scale) (break `/Game/1765/Systems/Inventory/Struct_Items` _returnvalue))
      (set `self.Item Description` _itemdescription)
      (`StaticMeshComponent.SetStaticMesh` _cube _mesh)
      (`SceneComponent.SetWorldScale3D` _cube (* (1.0 1.0 1.0) _scale))
      (for _array_element (`StaticMesh.StaticMaterials` _mesh)
        (`PrimitiveComponent.SetMaterial` _cube 0 (`.MaterialInterface` (break `StaticMaterial` _array_element)))))))

(fn `Interact With`
  (params (WhoIsInteracting :type "/Game/ThirdPerson/Blueprints/BP_ThirdPersonCharacter Object Reference"))
  (returns (Success :type Boolean))
  (`/Game/1765/Systems/Inventory/InventoryComponent.Add To Inventory` (`/Game/ThirdPerson/Blueprints/BP_ThirdPersonCharacter.InventoryComponent` WhoIsInteracting) (`self.ItemName`) (`self.Quantity`))
  (`self.K2_DestroyActor`)
  (return true))

(fn `Look At`
  (params (WhoIsLooking :type "/Game/ThirdPerson/Blueprints/BP_ThirdPersonCharacter Object Reference"))
  (returns (Message :type Text) (`Item Name` :type Name))
  (return (`self.Item Description`) (`self.ItemName`)))

(fn `UserConstructionScript`)