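; BP_ItemContainer is an interactable chest that holds items in its own InventoryComponent, seeded with a dagger at BeginPlay.
; Looking at it returns an "Open Chest" prompt, and interacting opens a DualInventory widget pairing the interactor's inventory with the container's, titled by the actor's display name.
; The widget reference is kept so ending any actor overlap closes the UI, a hack for detecting when the player leaves range.
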(event `self.ReceiveBeginPlay`
  (`/Game/1765/Systems/Inventory/InventoryComponent.Add To Inventory` (`self.InventoryComponent`) "dagger" 1))

(event `self.ReceiveActorEndOverlap`
  (params (OtherActor :type "Actor Object Reference"))
  (bind _dualinventory (`self.DualInventory`)
    (:`then`
      (`/Game/1765/Systems/Inventory/UI/DualInventory.CloseDualInventory` _dualinventory))
    (:`else`)))

(fn `Interact With`
  (params (WhoIsInteracting :type "/Game/ThirdPerson/Blueprints/BP_ThirdPersonCharacter Object Reference"))
  (returns (Success :type Boolean))
  (bind _returnvalue (`|CreateWidget` "/Game/1765/Systems/Inventory/UI/DualInventory.DualInventory_C" null (`/Game/ThirdPerson/Blueprints/BP_ThirdPersonCharacter.InventoryComponent` WhoIsInteracting) (`self.InventoryComponent`) (`KismetTextLibrary.Conv_StringToText` (`KismetSystemLibrary.GetDisplayName` self))))
  (set `self.DualInventory` _returnvalue)
  (`UserWidget.AddToViewport` _returnvalue 0)
  (return true))

(fn `Look At`
  (params (WhoIsLooking :type "/Game/ThirdPerson/Blueprints/BP_ThirdPersonCharacter Object Reference"))
  (returns (Message :type Text) (`Item Name` :type Name))
  (return "Open Chest" "None"))

(fn `UserConstructionScript`)