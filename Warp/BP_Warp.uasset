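; BP_Warp is a portal actor that teleports the player character to a linked portal's exit point when a BP_ThirdPersonCharacter overlaps it.
; Its construction script finds the BP_Warp whose PortalID matches ExitPortalID and can display the route as debug text.
; On overlap it applies the exit's location and rotation, or prints a warning if unlinked.
; BlastOutExit optionally adds a fixed world-space launch, pop sound and unpaused blast VFX.
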(event `self.ReceiveActorBeginOverlap`
  (params (OtherActor :type "Actor Object Reference"))
  (bind _returnvalue (`GameplayStatics.GetPlayerCharacter` 0))
  (bind _returnvalue_2 (`self.GetTransform`))
  (bind _exit (`/Warp/BP_Warp.Exit` (`self.ExitPortal`)))
  (cast `/Game/ThirdPerson/Blueprints/BP_ThirdPersonCharacter` OtherActor)
  (if (`self.DebugHasExist?`)
    (`self.K2_SetActorLocationAndRotation` _returnvalue (`SceneComponent.K2_GetComponentLocation` _exit) (`KismetMathLibrary.TransformRotation` _returnvalue_2 (`KismetMathLibrary.InverseTransformRotation` _returnvalue_2 (`SceneComponent.K2_GetComponentRotation` _exit))) false false)
    (if (`self.BlastOutExit?`)
      (`Character.LaunchCharacter` _returnvalue (900.0 0.0 100.0) true true)
      (`GameplayStatics.PlaySound2D` "/Game/Interface_And_Item_Sounds/WAV/Abstract_Pop_02.Abstract_Pop_02" 1.0 1.0 0.0 null null)
      (`NiagaraComponent.SetPaused` (`self.BlastVFX`) false))
    (else
      (`KismetSystemLibrary.PrintString` "Broken Portal!!!"))))

(fn `UserConstructionScript`
  (bind _outactors (`GameplayStatics.GetAllActorsOfClass` "BP_Warp_C"))
  (for _array_element _outactors
    (if (== (`/Warp/BP_Warp.PortalID` _array_element) (`self.ExitPortalID`))
      (set `self.DebugHasExist?` true)
      (set `self.ExitPortal` _array_element)))
  (if (`self.DebugDisplayRoute?`)
    (`TextRenderComponent.K2_SetText` (`self.DebugText`) (`KismetTextLibrary.Conv_StringToText` (`KismetStringLibrary.Concat_StrStr` "ID: " (`KismetStringLibrary.Conv_IntToString` (`self.PortalID`)) "Exit: " (`KismetStringLibrary.Conv_IntToString` (`self.ExitPortalID`)) "Valid Exit? " (`KismetStringLibrary.Conv_BoolToString` (`self.DebugHasExist?`)))))))